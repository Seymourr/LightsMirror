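; Player pawn for a grid-based laser puzzle, handling mouse placement, pickup, removal and rotation (hold R) of Reflectors and Splitters.
; On BeginPlay it spawns the StartLaser on an edge cell of the level's tile map.
; Mouse positions map to grid cells, allowing for camera black bars and the sidebar's screen share.
; Held pieces snap to cells each tick, hiding when blocked or off-grid, while the sidebar menu tracks piece counts.
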(event EventBeginPlay
  (bind _returnvalue (Game|GetPlayerController 0))
  (bind _outactors (Actor|GetAllActorsOfClass "/Script/Engine.CameraActor"))
  (bind _array_element (Utilities|Array|ForEachLoopwithBreak _outactors :!label _label)
    (:LoopBody
      (if (Actor|ActorHasTag _array_element "MainCamera")
        (Variables|Default|SetMainCamera _array_element)
        (goto _label Break)))
    (:Completed
      ;[1 1 1] Initialization
      (Input|SetInputModeGameandUI _returnvalue (Variables|Default|GetMenu) false false)
      (Variables|/Script/Engine.PlayerController|SetbShowMouseCursor _returnvalue true)
      (Variables|Default|SetHeldObject (Variables|Default|GetNullObject))
      (bind (_mapwidth _mapheight _levelwidth _levelheight) (CallFunction|GetLevelDims))
      (CallFunction|SpawnPlacable "/Game/Blocks/StartLaser.StartLaser_C" (Math|Conversions|ToTransform(Vector) (Utilities|ConvertGridPositiontoLevelPosition (- _mapwidth 1) (/ _mapheight 2) _mapwidth _mapheight 0.0 _levelheight _levelwidth _levelheight))))))

(event EventTick
  (params (DeltaSeconds :type Float%20%28single-precision%29))
  ;[1 1 1] User Interaction
  (CallFunction|UpdateHeldLocation))

(event Input|MouseEvents|RightMouseButton
  (params (Key :type Key%20Structure :default "AnyKey"))
  ;[1 1 1] User Interaction
  (:Pressed
    (CallFunction|RemovePlaced)))

(event Input|KeyboardEvents|R
  (params (Key :type Key%20Structure :default "AnyKey"))
  ;[1 1 1] User Interaction
  (:Pressed
    (bind _output_get (Variables|Default|SetHolding true))
    (CallFunction|RotateObject :!label _label)
    (if _output_get
      (Utilities|FlowControl|Delay 0.05)
      (goto _label)))
  (:Released
    (Variables|Default|SetHolding false)))

(event Input|MouseEvents|LeftMouseButton
  (params (Key :type Key%20Structure :default "AnyKey"))
  ;[1 1 1] User Interaction
  (:Pressed
    (CallFunction|PlaceorPickUp)))

(fn ConstructionScript
  (bind _outactors (Actor|GetAllActorsOfClass "/Game/Sprites/B_Level0.B_Level0_C"))
  (Variables|Default|SetTileMap (Variables|/Game/Sprites/B_Level0.B_Level0_C|Getlevel0 (Utilities|Array|Get(acopy) _outactors)))
  (bind _assidebar (Utilities|Casting|CastTosidebar (UserInterface|GetUserWidgetObject (Variables|/Game/Sprites/B_Level0.B_Level0_C|Getsidebar (Utilities|Array|Get(acopy) _outactors)))))
  (Variables|Default|SetMenu _assidebar))

(fn SetLaser
  (params (Source :type Vector) (Target :type Vector) (Laser :type Particle%20System%20Component%20Object%20Reference))
  (Effects|Components|ParticleSystem|SetVectorParameter Laser "BeamSource" Source)
  (Effects|Components|ParticleSystem|SetVectorParameter Laser "BeamTarget" (+ Target (+ (Math|Float|Truncate (Math|Vector|VectorLength (- Source Target))) (LocalVariables|Getoffset)))))

(fn GetActorsatGridLocation
  (params (GridX :type Integer) (GrixY :type Integer))
  (bind _accumelatedactors (LocalVariables|GetAccumelatedActors))
  (bind (_mapwidth _mapheight _levelwidth _levelheight) (CallFunction|GetLevelDims))
  (Utilities|Array|Clear _accumelatedactors)
  (Utilities|Array|Clear (Variables|Default|GetCloseActors))
  (bind _outactors (Actor|GetAllActorsOfClass "/Game/Blocks/Reflector.Reflector_C"))
  (for _array_element _outactors
    (Utilities|Array|Add _accumelatedactors _array_element))
  (bind _outactors_2 (Actor|GetAllActorsOfClass "/Game/Blocks/Splitter.Splitter_C"))
  (for _array_element_2 _outactors_2
    (Utilities|Array|Add _accumelatedactors _array_element_2))
  (bind _outactors_3 (Actor|GetAllActorsOfClass "/Game/Blocks/StartLaser.StartLaser_C"))
  (for _array_element_3 _outactors_3
    (Utilities|Array|Add _accumelatedactors _array_element_3))
  (for _array_element_4 _accumelatedactors
    (if (and (== (.GridX (Utilities|ConvertLevelPositiontoGridPosition (Transformation|GetActorLocation _array_element_4) _mapwidth _mapheight _levelwidth _levelheight)) GridX) (== (.GridY (Utilities|ConvertLevelPositiontoGridPosition (Transformation|GetActorLocation _array_element_4) _mapwidth _mapheight _levelwidth _levelheight)) GrixY))
      (Utilities|Array|Add (Variables|Default|GetCloseActors) _array_element_4)))
  (return (Variables|Default|GetCloseActors)))

(fn DisableActor
  (params (Actor :type Actor%20Object%20Reference))
  (Input|DisableInput Actor (Game|GetPlayerController 0))
  (Rendering|SetActorHiddenInGame Actor true)
  (Actor|Tick|SetActorTickEnabled Actor true))

(fn EnableActor
  (params (Actor :type Actor%20Object%20Reference))
  (Input|EnableInput Actor (Game|GetPlayerController 0))
  (Rendering|SetActorHiddenInGame Actor false)
  (Actor|Tick|SetActorTickEnabled Actor))

(fn GetLevelDims
  (bind _tilemap (Variables|Default|GetTileMap))
  (bind _boxextent (Collision|GetComponentBounds _tilemap))
  (bind (_x _y _z) (Math|Vector|BreakVector _boxextent))
  (bind (_mapwidth _mapheight) (Class|PaperTileMapComponent|GetMapSize _tilemap))
  (return _mapwidth _mapheight (* _y 2.0) (* _z -2.0)))

(fn GetGridDims
  (bind _returnvalue (Viewport|GetViewportSize))
  (bind (_x _y) (Math|Vector2D|BreakVector2D _returnvalue))
  (bind (_blackbarwidth _blackbarheight) (CallFunction|GetBlackBarSize))
  (return (+ (* (- _x (* _blackbarwidth 2.0)) 0.755) (* _blackbarwidth 2.0)) (+ (* (- _y (* _blackbarheight 2.0)) 1.0) (* _blackbarheight 2.0))))

(fn UpdateHeldLocation
  (bind _returnvalue (Game|GetPlayerController 0))
  (bind _heldobject (Variables|Default|GetHeldObject))
  (bind (_locationx _locationy) (Game|Player|GetMousePosition _returnvalue))
  ;[1 1 1] Make a held object follow the mouse cursors location. If above another actor, hide the held object.
  ;;[1 1 1] Is an object held?
  (if (not (== (Variables|Default|GetHeldObject) (Variables|Default|GetNullObject)))
    (bind (_mapwidth _mapheight _levelwidth _levelheight) (CallFunction|GetLevelDims))
    (bind (_blackbarwidth _blackbarheight) (CallFunction|GetBlackBarSize))
    (bind (_width _height) (CallFunction|GetGridDims))
    (Transformation|SetActorLocation _heldobject (Utilities|ConvertGridPositiontoLevelPosition (.GridX (Utilities|ConvertScreenPositiontoGridPosition (Math|Vector2D|MakeVector2D _locationx _locationy) _mapwidth _mapheight _width _height _blackbarwidth _blackbarheight)) (.GridY (Utilities|ConvertScreenPositiontoGridPosition (Math|Vector2D|MakeVector2D _locationx _locationy) _mapwidth _mapheight _width _height _blackbarwidth _blackbarheight)) _mapwidth _mapheight 0.0 _levelheight _levelwidth _levelheight) false false)
    (bind _actors (CallFunction|GetActorsatGridLocation (.GridX (Utilities|ConvertScreenPositiontoGridPosition (Math|Vector2D|MakeVector2D _locationx _locationy) _mapwidth _mapheight _width _height _blackbarwidth _blackbarheight)) (.GridY (Utilities|ConvertScreenPositiontoGridPosition (Math|Vector2D|MakeVector2D _locationx _locationy) _mapwidth _mapheight _width _height _blackbarwidth _blackbarheight))))
    (if (or (== (Utilities|Array|Length _actors) 2) (Math|Boolean|ORBoolean (>= (.GridX (Utilities|ConvertScreenPositiontoGridPosition (Math|Vector2D|MakeVector2D _locationx _locationy) _mapwidth _mapheight _width _height _blackbarwidth _blackbarheight)) _mapwidth) (< (.GridX (Utilities|ConvertScreenPositiontoGridPosition (Math|Vector2D|MakeVector2D _locationx _locationy) _mapwidth _mapheight _width _height _blackbarwidth _blackbarheight)) 0) (>= (.GridY (Utilities|ConvertScreenPositiontoGridPosition (Math|Vector2D|MakeVector2D _locationx _locationy) _mapwidth _mapheight _width _height _blackbarwidth _blackbarheight)) _mapheight) (< (.GridY (Utilities|ConvertScreenPositiontoGridPosition (Math|Vector2D|MakeVector2D _locationx _locationy) _mapwidth _mapheight _width _height _blackbarwidth _blackbarheight)) 0)))
      (CallFunction|DisableActor _heldobject)
      (else
        (CallFunction|EnableActor _heldobject)))))

(fn RemovePlaced
  (bind _returnvalue (Game|GetPlayerController 0))
  (bind _menu (Variables|Default|GetMenu))
  (bind (_locationx _locationy) (Game|Player|GetMousePosition _returnvalue))
  ;[1 1 1] Removes the object located under the mouse, if there is one.
  (bind (_blackbarwidth _blackbarheight) (CallFunction|GetBlackBarSize))
  (bind (_mapwidth _mapheight) (CallFunction|GetLevelDims))
  (bind (_width _height) (CallFunction|GetGridDims))
  (bind _actors (CallFunction|GetActorsatGridLocation (.GridX (Utilities|ConvertScreenPositiontoGridPosition (Math|Vector2D|MakeVector2D _locationx _locationy) _mapwidth _mapheight _width _height _blackbarwidth _blackbarheight)) (.GridY (Utilities|ConvertScreenPositiontoGridPosition (Math|Vector2D|MakeVector2D _locationx _locationy) _mapwidth _mapheight _width _height _blackbarwidth _blackbarheight))))
  (for _array_element _actors
    (LocalVariables|SetClass (Utilities|GetClass _array_element))
    (if (not (== _array_element (Variables|Default|GetHeldObject)))
      (Actor|DestroyActor _array_element)
      (if (== (LocalVariables|GetClass) "/Game/Blocks/Reflector.Reflector_C")
        (Default|RemoveCreated _menu false)
        (elif (== (LocalVariables|GetClass) "/Game/Blocks/Splitter.Splitter_C")
          (Default|RemoveCreated _menu false 1))))))

(fn PlaceorPickUp
  (bind _returnvalue (Game|GetPlayerController 0))
  (bind _menu (Variables|Default|GetMenu))
  (bind _menu_2 (Variables|Default|GetMenu))
  (bind (_locationx _locationy) (Game|Player|GetMousePosition _returnvalue))
  (bind (_blackbarwidth _blackbarheight) (CallFunction|GetBlackBarSize))
  (bind (_mapwidth _mapheight _levelwidth _levelheight) (CallFunction|GetLevelDims))
  (bind (_width _height) (CallFunction|GetGridDims))
  (if (and (and (>= (Math|Conversions|ToFloat(Integer) (.GridX (Utilities|ConvertScreenPositiontoGridPosition (Math|Vector2D|MakeVector2D _locationx _locationy) _mapwidth _mapheight _width _height _blackbarwidth _blackbarheight))) 0.0) (< (.GridX (Utilities|ConvertScreenPositiontoGridPosition (Math|Vector2D|MakeVector2D _locationx _locationy) _mapwidth _mapheight _width _height _blackbarwidth _blackbarheight)) _mapwidth)) (and (>= (Math|Conversions|ToFloat(Integer) (.GridY (Utilities|ConvertScreenPositiontoGridPosition (Math|Vector2D|MakeVector2D _locationx _locationy) _mapwidth _mapheight _width _height _blackbarwidth _blackbarheight))) 0.0) (< (.GridY (Utilities|ConvertScreenPositiontoGridPosition (Math|Vector2D|MakeVector2D _locationx _locationy) _mapwidth _mapheight _width _height _blackbarwidth _blackbarheight)) _mapheight)))
    (bind _actors (CallFunction|GetActorsatGridLocation (.GridX (Utilities|ConvertScreenPositiontoGridPosition (Math|Vector2D|MakeVector2D _locationx _locationy) _mapwidth _mapheight _width _height _blackbarwidth _blackbarheight)) (.GridY (Utilities|ConvertScreenPositiontoGridPosition (Math|Vector2D|MakeVector2D _locationx _locationy) _mapwidth _mapheight _width _height _blackbarwidth _blackbarheight))))
    (bind _output_get (LocalVariables|SetClass (Utilities|GetClass (Variables|Default|GetHeldObject))))
    (if (== (Utilities|Array|Length _actors) 1)
      (if (== (Variables|Default|GetHeldObject) (Variables|Default|GetNullObject))
        (if (== (Utilities|GetClass (Utilities|Array|Get(acopy) _actors)) "/Game/Blocks/Reflector.Reflector_C")
          (Default|RemoveCreated _menu false)
          (bind _asreflector (Utilities|Casting|CastToReflector (Utilities|Array|Get(acopy) _actors)))
          (Effects|Components|ParticleSystem|SetVectorParameter (Variables|/Game/Blocks/Reflector.Reflector_C|GetPar_Beam _asreflector) "BeamTarget" "0, 0, 0")
          (bind _output_get_2 (Variables|Default|SetHeldObject (Utilities|Array|Get(acopy) _actors) :!label _label))
          (Collision|SetActorEnableCollision _output_get_2 false)
          (CallFunction|AddShield _output_get_2)
          (elif (== (Utilities|GetClass (Utilities|Array|Get(acopy) _actors)) "/Game/Blocks/Splitter.Splitter_C")
            (Default|RemoveCreated _menu false 1)
            ;[1 1 1] TODO: Same for splitter
            (Utilities|Casting|CastToSplitter (Utilities|Array|Get(acopy) _actors))
            (goto _label)))
        (else
          (Actor|DestroyActor (Variables|Default|GetHeldObject))
          (bind _created (CallFunction|SpawnPlacable _output_get (Math|Conversions|ToTransform(Vector) (Utilities|ConvertGridPositiontoLevelPosition (.GridX (Utilities|ConvertScreenPositiontoGridPosition (Math|Vector2D|MakeVector2D _locationx _locationy) _mapwidth _mapheight _width _height _blackbarwidth _blackbarheight)) (.GridY (Utilities|ConvertScreenPositiontoGridPosition (Math|Vector2D|MakeVector2D _locationx _locationy) _mapwidth _mapheight _width _height _blackbarwidth _blackbarheight)) _mapwidth _mapheight 0.0 _levelheight _levelwidth _levelheight))))
          (Collision|SetActorEnableCollision _created true)
          (Variables|Default|SetHeldObject (Variables|Default|GetNullObject))
          (if (== (Utilities|GetClass _created) "/Game/Blocks/Reflector.Reflector_C")
            (Default|AddCreated _menu_2)
            (elif (== (Utilities|GetClass _created) "/Game/Blocks/Splitter.Splitter_C")
              (Default|AddCreated _menu_2 1))))))))

(fn OLD)

(fn RotateObject
  (bind _returnvalue (Game|GetPlayerController 0))
  (bind _rotationamount (Variables|Default|GetRotationAmount))
  (bind (_locationx _locationy) (Game|Player|GetMousePosition _returnvalue))
  (bind (_blackbarwidth _blackbarheight) (CallFunction|GetBlackBarSize))
  (Variables|Default|SetHoverObject (Variables|Default|GetNullObject))
  (bind (_mapwidth _mapheight) (CallFunction|GetLevelDims))
  (bind (_width _height) (CallFunction|GetGridDims))
  (bind _actors (CallFunction|GetActorsatGridLocation (.GridX (Utilities|ConvertScreenPositiontoGridPosition (Math|Vector2D|MakeVector2D _locationx _locationy) _mapwidth _mapheight _width _height _blackbarwidth _blackbarheight)) (.GridY (Utilities|ConvertScreenPositiontoGridPosition (Math|Vector2D|MakeVector2D _locationx _locationy) _mapwidth _mapheight _width _height _blackbarwidth _blackbarheight))))
  (for _array_element _actors
    (if (not (== _array_element (Variables|Default|GetHeldObject)))
      (Variables|Default|SetHoverObject _array_element)))
  (if (Utilities|IsValid (Variables|Default|GetHoverObject))
    (Utilities|Casting|CastToStartLaser (Variables|Default|GetHoverObject)
      (:CastFailed
        (Class|Actor|AddActorWorldRotation (Variables|Default|GetHoverObject) (Math|Rotator|MakeRotator (Variables|Default|GetRotationAmount) 0.0 0.0))))
    (elif (Utilities|IsValid (Variables|Default|GetHeldObject))
      (Variables|Default|SetCurrentRotation (Math|Float|%(Float) (+ (Variables|Default|GetCurrentRotation) _rotationamount) 3.6e+02))
      (Class|Actor|AddActorWorldRotation (Variables|Default|GetHeldObject) (Math|Rotator|MakeRotator _rotationamount 0.0 0.0)))))

(fn SpawnPlacable
  (params (class :type Actor%20Class%20Reference) (pos :type Transform))
  (bind _returnvalue (Game|SpawnActorfromClass class pos "Undefined" 0 0))
  (Transformation|SetActorRotation _returnvalue "0.000000,90.000000,0.000000")
  (Class|Actor|AddActorWorldRotation _returnvalue (Math|Rotator|MakeRotator (Variables|Default|GetCurrentRotation) 0.0 0.0))
  (Transformation|SetActorScale3D _returnvalue "0.238594,0.242728,0.242728")
  (return _returnvalue))

(fn GetBlackBarSize
  (bind _returnvalue (Viewport|GetViewportSize))
  (bind _returnvalue_2 (Viewport|GetViewportSize))
  (bind _maincamera (Variables|Default|GetMainCamera))
  (bind (_x _y) (Math|Vector2D|BreakVector2D _returnvalue))
  (bind (_x_2 _y_2) (Math|Vector2D|BreakVector2D _returnvalue_2))
  (bind _cameracomponent (Variables|/Script/Engine.CameraActor|GetCameraComponent _maincamera))
  (bind _returnvalue_3 (/ _x _y))
  (bind _aspectratio (Variables|/Script/Engine.CameraComponent|GetAspectRatio _cameracomponent))
  (if (> _aspectratio _returnvalue_3)
    (return 0.0 (/ (* _y_2 (- 1.0 (/ _returnvalue_3 _aspectratio))) 2.0))
    (else
      (return (/ (* _x_2 (- 1.0 (/ _aspectratio _returnvalue_3))) 2.0) 0.0))))

(fn AddShield
  (params (Target :type Actor%20Object%20Reference))
  (bind _returnvalue (AddComponent|AddSceneComponent Target false))
  (bind _returnvalue_2 (Effects|SpawnEmitterAttached "/Game/Beam/OrbitSelect.OrbitSelect" _returnvalue "None" "0,0.000000, 0" "0.000000,0.000000,90.000000"))
  (Transformation|SetWorldScale3D _returnvalue_2 "0.100000,0.100000, 0")
  (return))
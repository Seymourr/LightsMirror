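; Enemy spawner actor that repeatedly spawns a configurable character class around its own location.
; On BeginPlay, a looping timer calls SpawnEnemy at the TimeOffset interval.
; Each spawn adds random Y and Z offsets derived from SpawnOffset, keeping the spawner's X and scale and adding 90 degrees of pitch to its rotation.
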(event EventBeginPlay
  (Utilities|Time|SetTimerbyFunctionName 0 "SpawnEnemy" (Variables|Default|GetTimeOffset) true))

(fn ConstructionScript)

(fn SpawnEnemy
  (bind _returnvalue (Transformation|GetActorTransform))
  (bind _spawnoffset (Variables|Default|GetSpawnOffset))
  (bind (_location _rotation _scale) (Math|Transform|BreakTransform _returnvalue))
  (bind (_roll _pitch _yaw) (Math|Rotator|BreakRotator _rotation))
  (bind (_x _y _z) (Math|Vector|BreakVector _location))
  (Game|SpawnActorfromClass (Variables|Default|GetTargerCharacter) (Math|Transform|MakeTransform (Math|Vector|MakeVector _x (+ _y (Math|Random|RandomFloatinRange (stale _result) _spawnoffset)) (+ (Math|Random|RandomFloatinRange (stale _result) _spawnoffset) _z)) (Math|Rotator|MakeRotator _roll (+ _pitch 9e+01) _yaw) _scale) "Undefined" 0 0)
  (return))
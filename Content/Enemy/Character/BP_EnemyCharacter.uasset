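; Enemy thief character that steals treasure and carries it to an exit node, costing the player a life.
; Tick seeks the nearest available Treasure, attaches it on contact, then heads for the closest TargetNode and destroys both on arrival.
; Movement steers straight at the target through AddMovementInput, without pathfinding.
; DoDamage uses a brief Tick-reset hit cooldown and drops carried treasure on death; an HP widget references the enemy.
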(event EventBeginPlay
  (Variables|Default|SetCurHealth (Variables|Default|GetMaxHealth))
  (bind _asenemy_hpwidget (Utilities|Casting|CastToEnemyHPWidget (UserInterface|GetUserWidgetObject (Variables|Default|GetWidget))))
  (Variables|/Game/Enemy/UMG/EnemyHPWidget.EnemyHPWidget_C|SetPlayer _asenemy_hpwidget self))

(event EventTick
  (params (DeltaSeconds :type Float%20%28single-precision%29))
  (if (Variables|Default|GetstartTimer)
    (Variables|Default|SetstartTimer false)
    (Utilities|FlowControl|Delay 0.01)
    (Variables|Default|SetCanHit true))
  (if (Variables|Default|GetInPossessionOfTreasue)
    ;[1 1 1] Move towards target with ze loot
    (bind _closesttarget2 (CallFunction|GetClosestTarget (Transformation|GetActorLocation) :!label _label))
    (CallFunction|MoveTowards DeltaSeconds _closesttarget2)
    (if (< (Transformation|GetDistanceTo _closesttarget2) 4e+01)
      (Audio|PlaySound2D "/Game/Sounds/kaching.kaching")
      (bind _asmain_pawn (Utilities|Casting|CastToMainPawn (Game|Player|GetPlayerPawn 0)))
      (Default|LifeLoss _asmain_pawn)
      (Actor|DestroyActor (Variables|Default|GetPossessedTreasure))
      (Actor|DestroyActor))
    (else
      ;[1 1 1] Valid target check
      (if (Utilities|IsValid (Variables|Default|GetDesiredTarget))
        (if (Variables|/Game/Enemy/Blueprints/Treasure.Treasure_C|GetisAvailable (Variables|Default|GetDesiredTarget))
          ;[1 1 1] Close enough to grab check
          (if (< (Transformation|GetDistanceTo (Variables|Default|GetDesiredTarget)) 4e+01)
            ;[1 1 1] After grab sets
            (Variables|/Game/Enemy/Blueprints/Treasure.Treasure_C|SetisAvailable (Variables|Default|GetDesiredTarget) false)
            (Variables|Default|SetInPossessionOfTreasue true)
            (bind _output_get (Variables|Default|SetPossessedTreasure (Variables|Default|GetDesiredTarget)))
            (Transformation|AttachActorToActor _output_get self "None" "KeepRelative" "KeepRelative" "KeepRelative" true)
            (Transformation|SetActorRelativeLocation _output_get "0.000000, 0,-15.000000")
            (Transformation|SetActorRelativeRotation _output_get "0.000000, 0,90.000000")
            (Transformation|SetActorRelativeScale3D _output_get "0.600000,0.600000,0.600000")
            (Audio|PlaySound2D "/Game/Sounds/Evil_Laugh_2-Sound_Explorer-1081271267.Evil_Laugh_2-Sound_Explorer-1081271267")
            (goto _label)
            (else
              (CallFunction|MoveTowards DeltaSeconds (Variables|Default|GetDesiredTarget))))
          (else
            ;[1 1 1] Valid target search
            (bind _closesttarget2_2 (CallFunction|GetClosestTreasure (Transformation|GetActorLocation) :!label _label_2))
            (Variables|Default|SetDesiredTarget _closesttarget2_2)))
        (else
          (goto _label_2))))))

(fn ConstructionScript)

(fn GetClosestTreasure
  (params (AI_Location :type Vector))
  (bind _outactors (Actor|GetAllActorsOfClass "/Game/Enemy/Blueprints/Treasure.Treasure_C"))
  (for _array_element _outactors
    (if (Variables|/Game/Enemy/Blueprints/Treasure.Treasure_C|GetisAvailable _array_element)
      (if (or (< (Math|Vector|VectorLength (- AI_Location (Transformation|GetActorLocation _array_element))) (LocalVariables|GetClosestTargetDistance)) (== (LocalVariables|GetClosestTargetDistance) 0.0))
        (LocalVariables|SetClosestTargetDistance (Math|Vector|VectorLength (- AI_Location (Transformation|GetActorLocation _array_element))))
        (LocalVariables|SetClosestTarget _array_element))))
  (return (LocalVariables|GetClosestTarget)))

(fn MoveTowards
  (params (Delta :type Float%20%28single-precision%29) (Target :type Actor%20Object%20Reference))
  (bind _returnvalue (Transformation|GetActorLocation Target))
  (bind _self self)
  (bind _returnvalue_2 (Transformation|GetActorLocation _self))
  (Pawn|Input|AddMovementInput (Math|Vector|Normalize (- _returnvalue _returnvalue_2)) (* Delta (Variables|Default|GetMySpeed)) false)
  (Transformation|SetActorRotation _self (Math|Rotator|MakeRotator (* (.Yaw (Math|Rotator|BreakRotator (Math|Rotator|FindLookatRotation _returnvalue_2 _returnvalue))) 3.0) 0.0 0.0))
  (return))

(fn GetClosestTarget
  (params (AI_Location :type Vector))
  (bind _outactors (Actor|GetAllActorsOfClass "/Game/Enemy/Blueprints/TargetNode.TargetNode_C"))
  (for _array_element _outactors
    (if (or (< (Math|Vector|VectorLength (- AI_Location (Transformation|GetActorLocation _array_element))) (LocalVariables|GetClosestTargetDistance)) (== (LocalVariables|GetClosestTargetDistance) 0.0))
      (LocalVariables|SetClosestTargetDistance (Math|Vector|VectorLength (- AI_Location (Transformation|GetActorLocation _array_element))))
      (LocalVariables|SetClosestTarget _array_element)))
  (return (LocalVariables|GetClosestTarget)))

(fn DoDamage
  (bind _possessedtreasure (Variables|Default|GetPossessedTreasure))
  (if (Variables|Default|GetCanHit)
    (Variables|Default|SetCanHit false)
    (Variables|Default|SetstartTimer true)
    (bind _output_get (Variables|Default|SetCurHealth (- (Variables|Default|GetCurHealth) 1.0)))
    (if (< _output_get 0.0)
      (if (Variables|Default|GetInPossessionOfTreasue)
        (Transformation|DetachFromActor _possessedtreasure "KeepRelative" "KeepRelative" "KeepRelative")
        (Transformation|SetActorLocation _possessedtreasure (Transformation|GetActorLocation self) false false)
        (Transformation|SetWorldScale3D (Variables|/Game/Enemy/Blueprints/Treasure.Treasure_C|GetDefaultSceneRoot _possessedtreasure) "1.000000,1.000000,1.000000")
        (Variables|/Game/Enemy/Blueprints/Treasure.Treasure_C|SetisAvailable _possessedtreasure true))
      (Audio|PlaySound2D "/Game/Sounds/Male_Grunt-SoundBible.Male_Grunt-SoundBible")
      (Actor|DestroyActor))))